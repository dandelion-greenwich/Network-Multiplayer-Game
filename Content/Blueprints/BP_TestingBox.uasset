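; BP_TestingBox is a test Blueprint that displays network authority and the value of a variable named ReplicatedVar.
; On BeginPlay it checks HasAuthority and writes the result to AuthorityText.
; Every Tick it converts ReplicatedVar to text and pushes it to VarText, with no logic in these graphs changing the value.
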(event EventBeginPlay
  (if (Ability|HasAuthority)
    (Rendering|Components|TextRender|SetText (Variables|Default|GetAuthorityText) (Utilities|Text|MakeLiteralText "Has authority"))
    (else
      (Rendering|Components|TextRender|SetText (Variables|Default|GetAuthorityText) (Utilities|Text|MakeLiteralText "Doesn't have authority")))))

(event EventTick
  (params (DeltaSeconds :type Float%20%28single-precision%29))
  (Rendering|Components|TextRender|SetText (Variables|Default|GetVarText) (Utilities|Text|MakeLiteralText (Utilities|Text|ToText(Float) (Variables|Default|GetReplicatedVar) "HalfToEven"))))

(fn ConstructionScript)